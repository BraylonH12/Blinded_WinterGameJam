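; Test object actor in BlueLight_Objects whose cube is shown or hidden by the blue light of BP_BlindedCharacter.
; Test_Collision overlaps with the character's BlueLightCollision set Seen if the light can hit and has hit something, and clear it on exit.
; Tick runs ItemVisibility, which applies Seen to the cube only while both light flags are true, otherwise leaving visibility unchanged.
; Show_Item and Hide_Item are empty.
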(event OnComponentBeginOverlap(test_Collision)
  (params (OverlappedComponent :type Primitive%20Component%20Object%20Reference) (OtherActor :type Actor%20Object%20Reference) (OtherComp :type Primitive%20Component%20Object%20Reference) (OtherBodyIndex :type Integer) (bFromSweep :type Boolean) (SweepResult :type Hit%20Result%20Structure%20%28by%20ref%29))
  (bind _returnvalue (Actor|GetActorOfClass "/Game/BP_BlindedCharacter.BP_BlindedCharacter_C"))
  (if (== (Variables|/Game/BP_BlindedCharacter.BP_BlindedCharacter_C|GetblueLight_Collision _returnvalue) OtherComp)
    (bind _returnvalue_2 (Actor|GetActorOfClass "/Game/BP_BlindedCharacter.BP_BlindedCharacter_C"))
    (if (and (Variables|/Game/BP_BlindedCharacter.BP_BlindedCharacter_C|GetblueLight_canHit _returnvalue_2) (Variables|/Game/BP_BlindedCharacter.BP_BlindedCharacter_C|GetblueLight_hitSomething _returnvalue_2))
      (Variables|Default|Setseen true))))

(event OnComponentEndOverlap(test_Collision)
  (params (OverlappedComponent :type Primitive%20Component%20Object%20Reference) (OtherActor :type Actor%20Object%20Reference) (OtherComp :type Primitive%20Component%20Object%20Reference) (OtherBodyIndex :type Integer))
  (bind _returnvalue (Actor|GetActorOfClass "/Game/BP_BlindedCharacter.BP_BlindedCharacter_C"))
  (if (== (Variables|/Game/BP_BlindedCharacter.BP_BlindedCharacter_C|GetblueLight_Collision _returnvalue) OtherComp)
    (Variables|Default|Setseen false)))

(event Custom|Show_Item)

(event Custom|Hide_Item)

(event EventBeginPlay
  (Variables|Default|Setseen false))

(event Collision|EventActorBeginOverlap
  (params (OtherActor :type Actor%20Object%20Reference)))

(event EventTick
  (params (DeltaSeconds :type Float%20%28single-precision%29))
  (CallFunction|ItemVisibility))

(fn ConstructionScript)

(fn ItemVisibility
  (bind _returnvalue (Actor|GetActorOfClass "/Game/BP_BlindedCharacter.BP_BlindedCharacter_C"))
  (if (and (Variables|/Game/BP_BlindedCharacter.BP_BlindedCharacter_C|GetblueLight_canHit _returnvalue) (Variables|/Game/BP_BlindedCharacter.BP_BlindedCharacter_C|GetblueLight_hitSomething _returnvalue))
    (if (Variables|Default|Getseen)
      (Rendering|SetVisibility (Variables|Default|GetCube) true false)
      (else
        (Rendering|SetVisibility (Variables|Default|GetCube) false false)))))