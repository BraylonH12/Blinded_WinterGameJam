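; Skulk enemy that chases the player on sight and plays a one-time jumpscare on reaching them.
; Pawn sensing starts an AI move toward the player, and a successful move triggers the scare once through a DoOnce.
; The scare plays an attack animation, waits briefly, destroys the enemy and then increments PlayerLives on BP_BlindedCharacter.
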(event OnSeePawn(PawnSensing)
  (params (Pawn :type Pawn%20Object%20Reference))
  (Variables|Default|SetseePlayer true)
  (Variables|Default|SetcompleteJumpscare false)
  (CallFunction|Follow))

(event Custom|Follow
  (if (Variables|Default|GetseePlayer)
    (AI|AIMoveTo self "0, 0, 0" (Game|GetPlayerCharacter 0) 5.0 false
      (:OnSuccess
        (Utilities|FlowControl|DoOnce false
          (:Completed
            (CallFunction|JumpScare)))))
    (else
      (Variables|Default|SetseePlayer false))))

(event Custom|JumpScare
  (Components|Animation|PlayAnimation (Variables|Character|GetMesh) "/Game/FAB_Downloads/Whisper/Animations/Anim_Whisper_Attack3.Anim_Whisper_Attack3" false)
  (Variables|Default|SetcompleteJumpscare true)
  (Utilities|FlowControl|Delay 2.0)
  (Actor|DestroyActor)
  (bind _returnvalue (Actor|GetActorOfClass "/Game/BP_BlindedCharacter.BP_BlindedCharacter_C"))
  (Variables|/Game/BP_BlindedCharacter.BP_BlindedCharacter_C|SetplayerLives _returnvalue (+ 1 (Variables|/Game/BP_BlindedCharacter.BP_BlindedCharacter_C|GetplayerLives _returnvalue)))
  (Variables|Default|Setskulk_Alive false))

(event EventBeginPlay
  (Variables|Default|Setskulk_Alive true))

(event Collision|EventActorBeginOverlap
  (params (OtherActor :type Actor%20Object%20Reference)))

(event EventTick
  (params (DeltaSeconds :type Float%20%28single-precision%29)))

(fn ConstructionScript)