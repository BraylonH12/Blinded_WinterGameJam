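; BP_skulkSpawn is a spawner that keeps a skulk enemy in the level.
; BeginPlay spawns a BP_skulkEnemy at the SpawnPoint component's transform.
; Every Tick polls the first skulk found through GetActorOfClass and, when its SkulkAlive is false, calls SpawnSkulk, which adjusts for collisions but always spawns.
; A door BeatGame check is left unconnected and never runs.
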(event Custom|Spawn%20Skulk
  (Game|SpawnActorfromClass "/Game/Blueprints/Enemy/BP_skulkEnemy.BP_skulkEnemy_C" (Transformation|GetWorldTransform (Variables|Default|Getspawn%20point)) "AdjustIfPossibleButAlwaysSpawn" "MultiplyWithRoot" 0 0))

(event EventBeginPlay
  (Game|SpawnActorfromClass "/Game/Blueprints/Enemy/BP_skulkEnemy.BP_skulkEnemy_C" (Transformation|GetWorldTransform (Variables|Default|Getspawn%20point)) "Undefined" "MultiplyWithRoot" 0 0))

(event Collision|EventActorBeginOverlap
  (params (OtherActor :type Actor%20Object%20Reference)))

(event EventTick
  (params (DeltaSeconds :type Float%20%28single-precision%29))
  (bind _returnvalue (Actor|GetActorOfClass "/Game/Blueprints/Enemy/BP_skulkEnemy.BP_skulkEnemy_C"))
  (if (not (Variables|/Game/Blueprints/Enemy/BP_skulkEnemy.BP_skulkEnemy_C|Getskulk_Alive _returnvalue))
    (CallFunction|SpawnSkulk)))

(fn ConstructionScript)