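; BP_Door is the exit door that the player must unlock with a key to win and escape.
; When its collision is overlapped by the BP_BlindedCharacter found in the level, it checks that character's KeyFound flag.
; With the key, it destroys the door, sets BeatGame, prints an escape message and removes the BP_skulkEnemy.
; Without the key, it only prints a prompt that one is needed.
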(event OnComponentBeginOverlap(door_collision)
  (params (OverlappedComponent :type Primitive%20Component%20Object%20Reference) (OtherActor :type Actor%20Object%20Reference) (OtherComp :type Primitive%20Component%20Object%20Reference) (OtherBodyIndex :type Integer) (bFromSweep :type Boolean) (SweepResult :type Hit%20Result%20Structure%20%28by%20ref%29))
  (bind _returnvalue (Actor|GetActorOfClass "/Game/BP_BlindedCharacter.BP_BlindedCharacter_C"))
  (if (== _returnvalue OtherActor)
    (if (Variables|/Game/BP_BlindedCharacter.BP_BlindedCharacter_C|GetkeyFound _returnvalue)
      (Actor|DestroyActor)
      (Variables|Default|SetbeatGame true)
      (Development|PrintString "You Escaped!!")
      (Actor|GetActorOfClass "/Game/Blueprints/Enemy/BP_skulkEnemy.BP_skulkEnemy_C")
      (Actor|DestroyActor)
      (else
        (Development|PrintString "Need Key")))))

(event EventBeginPlay)

(event Collision|EventActorBeginOverlap
  (params (OtherActor :type Actor%20Object%20Reference)))

(event EventTick
  (params (DeltaSeconds :type Float%20%28single-precision%29)))

(fn ConstructionScript)